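; BP_ChemistLab is an actor Blueprint that puts the Chemist UI widget on screen when play begins.
; BeginPlay creates and adds the widget to the viewport, sets game-and-UI input focused on it, and enables the mouse cursor with click and hover events.
; Unwired leftover nodes for Shift-based switching to game-only input and for UI-only input never execute.
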(event `self.ReceiveBeginPlay`
  (bind _returnvalue (`GameplayStatics.GetPlayerController` 0))
  (bind _returnvalue_2 (`|CreateWidget` "/Game/Blueprint/Chemist.Chemist_C" _returnvalue))
  (`UserWidget.AddToViewport` _returnvalue_2 0)
  (`WidgetBlueprintLibrary.SetInputMode_GameAndUIEx` _returnvalue _returnvalue_2)
  (set `PlayerController.bShowMouseCursor` true _returnvalue)
  (set `PlayerController.bEnableMouseOverEvents` true _returnvalue)
  (set `PlayerController.bEnableClickEvents` true _returnvalue))

(event `self.ReceiveTick`
  (params (DeltaSeconds :type "Float (single-precision)")))

(fn `UserConstructionScript`)